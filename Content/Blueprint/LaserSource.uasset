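; LaserSource is an actor that emits a laser beam and marks the TheBox actor it hits as powered directly by a laser source.
; On BeginPlay it spawns a Laser actor, then each Tick traces forward from LaserDirection and moves the beam end to the hit or maximum range.
; It tracks the hit box as ChildBox, clearing that link when the target changes, and destroys boxes in one particular status.
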(event EventTick
  (params (DeltaSeconds :type Float%20%28single-precision%29))
  (bind _laserdirection (Variables|Default|GetLaserDirection))
  (bind _returnvalue (Transformation|GetWorldLocation _laserdirection))
  (bind _output_get (Variables|Default|SetLaserEndPoint (+ _returnvalue (* (Math|Vector|GetForwardVector _laserdirection) 5e+03))))
  (bind (_outhit _returnvalue_2) (Collision|LineTraceByChannel _returnvalue _output_get "TraceTypeQuery1" false 0 "ForOneFrame"))
  (if _returnvalue_2
    (Variables|Default|SetLaserEndPoint (.Location (Collision|BreakHitResult _outhit)))
    (bind _asthe_box (Utilities|Casting|CastToTheBox (.HitActor (Collision|BreakHitResult _outhit)))
      (:then
        (Utilities|CheckBoxFormandNull _asthe_box
          (:IsNull
            _)
          (:IsNotNull
            (if (== (Variables|Default|GetChildBox) _asthe_box)
              _
              (else
                (Utilities|SetNullBoxandNoneSource)))))
        (switch Utilities|FlowControl|Switch|SwitchonLaserSourceEnum (Variables|/Game/Blueprint/TheBox.TheBox_C|GetLaserSource _asthe_box)
          (:NewEnumerator0
            (bind _output_get_2 (Variables|Default|SetChildBox _asthe_box :!label _label))
            (Variables|/Game/Blueprint/TheBox.TheBox_C|SetLaserSource _output_get_2 "NewEnumerator1"))
          (:NewEnumerator1
            _)
          (:NewEnumerator2
            (goto _label))))
      (:CastFailed
        (if (!= (Variables|Default|GetChildBox) (Variables|Default|GetNullBox)) :!label _label_2
          (Utilities|SetNullBoxandNoneSource))))
    (else
      (goto _label_2)))
  (Class|ParticleSystemComponent|SetBeamEndPoint (Variables|/Game/Blueprint/Laser.Laser_C|GetLaserBeam (Variables|Default|GetLaser)) 0 (Variables|Default|GetLaserEndPoint)))

(event EventBeginPlay
  (bind _returnvalue (Game|SpawnActorfromClass "/Game/Blueprint/Laser.Laser_C" (Math|Transform|MakeTransform (Transformation|GetActorLocation) "0, 0, 0" "1,1,1") "Undefined" 0 0))
  (Variables|Default|SetLaser _returnvalue))

(fn ConstructionScript)
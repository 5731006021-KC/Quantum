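; TheBox is a physics box that relays a laser, switches between light wood and heavy metal forms, and can be highlighted or thrown.
; It spawns an attached Laser actor, shown while LaserSource is set, and line-traces forward each Tick.
; A box hit by the beam becomes ChildBox and inherits a source, chaining beams until contact breaks.
; Wood boxes hit by the beam are destroyed through an added destructible component.
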(event EventTick
  (params (DeltaSeconds :type Float%20%28single-precision%29))
  (bind _laser (Variables|Default|GetLaser))
  (bind _laserdirection (Variables|Default|GetLaserDirection))
  (bind _returnvalue (Transformation|GetWorldLocation _laserdirection))
  (bind _laserbeam (Variables|/Game/Blueprint/Laser.Laser_C|GetLaserBeam _laser))
  (bind _returnvalue_2 (Rendering|IsVisible _laserbeam))
  (switch Utilities|FlowControl|Switch|SwitchonLaserSourceEnum (Variables|Default|GetLaserSource)
    (:NewEnumerator0
      (if _returnvalue_2
        (CallFunction|SetLaserInvisible)
        (if (!= (Variables|Default|GetNullBox) (Variables|Default|GetChildBox))
          (Variables|TheBox_C|SetLaserSource (Variables|Default|GetChildBox) "NewEnumerator0")
          (Variables|Default|SetChildBox (Variables|Default|GetNullBox)))))
    (:NewEnumerator1
      (if _returnvalue_2 :!label _label
        _
        (else
          (CallFunction|SetLaserVisible)))
      (bind _output_get (Variables|Default|SetLaserEndPoint (+ _returnvalue (* (Math|Vector|GetForwardVector _laserdirection) 5e+03))))
      (bind (_outhit _returnvalue_3) (Collision|LineTraceByChannel _returnvalue _output_get "TraceTypeQuery1" false 0 "None"))
      (if _returnvalue_3
        (Variables|Default|SetLaserEndPoint (.Location (Collision|BreakHitResult _outhit)))
        (bind _asthe_box (Utilities|Casting|CastToTheBox (.HitActor (Collision|BreakHitResult _outhit)))
          (:then
            (Utilities|CheckBoxFormandNull _asthe_box
              (:IsNull
                _)
              (:IsNotNull
                (if (== (Variables|Default|GetChildBox) _asthe_box)
                  _
                  (else
                    (Utilities|SetNullBoxandNoneSource)))))
            (switch Utilities|FlowControl|Switch|SwitchonLaserSourceEnum (Variables|TheBox_C|GetLaserSource _asthe_box)
              (:NewEnumerator0
                (bind _output_get_2 (Variables|Default|SetChildBox _asthe_box))
                (Variables|TheBox_C|SetLaserSource _output_get_2 "NewEnumerator2"))
              (:NewEnumerator1
                _)
              (:NewEnumerator2
                _)))
          (:CastFailed
            (if (!= (Variables|Default|GetChildBox) (Variables|Default|GetNullBox)) :!label _label_2
              (Utilities|SetNullBoxandNoneSource))))
        (else
          (goto _label_2)))
      (Class|ParticleSystemComponent|SetBeamEndPoint (Variables|/Game/Blueprint/Laser.Laser_C|GetLaserBeam (Variables|Default|GetLaser)) 0 (Variables|Default|GetLaserEndPoint)))
    (:NewEnumerator2
      (goto _label))))

(event EventBeginPlay
  (bind _returnvalue (Game|SpawnActorfromClass "/Game/Blueprint/Laser.Laser_C" (Math|Transform|MakeTransform (Transformation|GetActorLocation) "0, 0, 0" "1,1,1") "Undefined" 0 0))
  (bind _output_get (Variables|Default|SetLaser _returnvalue))
  (Transformation|AttachActorToActor _output_get self "None" "SnapToTarget" "SnapToTarget" "SnapToTarget" true))

(fn ConstructionScript)

(fn Highlight
  (Rendering|SetRenderCustomDepth (Variables|Components|GetBoxMesh) true))

(fn LowMass
  (Class|PrimitiveComponent|SetMassOverrideinKg (Variables|Components|GetBoxMesh) "None" 1e+02 true)
  (Physics|SetEnableGravity (Variables|Components|GetBoxMesh) true)
  (Rendering|Material|SetMaterial (Variables|Components|GetBoxMesh) 0 "/Game/Material/TheBoxWoodTexture/TheBoxWood_Glass_Mat.TheBoxWood_Glass_Mat")
  (Rendering|Material|SetMaterial (Variables|Components|GetBoxMesh) 1 "/Game/Material/TheBoxWoodTexture/TheBoxWood_Body_Mat.TheBoxWood_Body_Mat")
  (Physics|SetSimulatePhysics (Variables|Components|GetBoxMesh) true)
  (Variables|Default|SetTheBoxStatus "NewEnumerator2"))

(fn HighMass
  (Class|PrimitiveComponent|SetMassOverrideinKg (Variables|Components|GetBoxMesh) "None" 5e+03 true)
  (Physics|SetEnableGravity (Variables|Components|GetBoxMesh) true)
  (Rendering|Material|SetMaterial (Variables|Components|GetBoxMesh) 0 "/Game/Material/TheBoxMetalTexture/TheBoxMetal_Glass_Mat.TheBoxMetal_Glass_Mat")
  (Rendering|Material|SetMaterial (Variables|Components|GetBoxMesh) 1 "/Game/Material/TheBoxMetalTexture/TheBoxMetal_Body_Mat.TheBoxMetal_Body_Mat")
  (Physics|SetSimulatePhysics (Variables|Components|GetBoxMesh) true)
  (Variables|Default|SetTheBoxStatus "NewEnumerator0"))

(fn ThrowObj
  (params (Force :type Vector))
  (Physics|AddImpulse (Variables|Components|GetBoxMesh) Force "None" true))

(fn Destroy
  (bind _boxmesh (Variables|Components|GetBoxMesh))
  (Rendering|SetVisibility (Variables|Components|GetBoxMesh) false true)
  (Physics|SetSimulatePhysics _boxmesh false)
  (Collision|SetCollisionEnabled _boxmesh "NoCollision")
  (bind _returnvalue (AddComponent|AddDestructibleComponent false))
  (Class|DestructibleComponent|ApplyRadiusDamage _returnvalue 1.0 (Transformation|GetWorldLocation _returnvalue) 1.0 2e+03 true))

(fn DeHighlight
  (Rendering|SetRenderCustomDepth (Variables|Components|GetBoxMesh) false))

(fn SetLaserVisible
  (Rendering|SetVisibility (Variables|/Game/Blueprint/Laser.Laser_C|GetLaserBeam (Variables|Default|GetLaser)) true false))

(fn SetLaserInvisible
  (Rendering|SetVisibility (Variables|/Game/Blueprint/Laser.Laser_C|GetLaserBeam (Variables|Default|GetLaser)) false false))
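; Pressure button Blueprint that opens and closes a linked Door and toggles its own emissive glow.
; On BeginPlay it finds the Door whose DoorID matches its BottonID.
; Overlap begin and end on ButtonOverlaps drive open and close through two DoOnce gates that reset each other, so the actions alternate.
; Tick adds upward velocity to the physics-driven Button each frame, pushing it back up like a spring.
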(event OnComponentBeginOverlap(ButtonOverlaps)
  (params (OverlappedComponent :type Primitive%20Component%20Object%20Reference) (OtherActor :type Actor%20Object%20Reference) (OtherComp :type Primitive%20Component%20Object%20Reference) (OtherBodyIndex :type Integer) (bFromSweep :type Boolean) (SweepResult :type Hit%20Result%20Structure%20%28by%20ref%29))
  (Utilities|FlowControl|DoOnce false
    (:Completed
      (Default|OpenDoor (Variables|Default|GetDoorRef))
      (Rendering|Material|SetScalarParameterValueonMaterials (Variables|Default|GetButton) "Emissive" 1.0)
      (Rendering|Material|SetScalarParameterValueonMaterials (Variables|Default|GetButtonBase) "Emissive" 1.0)
      (CallFunction|ResetClose))))

(event OnComponentEndOverlap(ButtonOverlaps)
  (params (OverlappedComponent :type Primitive%20Component%20Object%20Reference) (OtherActor :type Actor%20Object%20Reference) (OtherComp :type Primitive%20Component%20Object%20Reference) (OtherBodyIndex :type Integer))
  (Utilities|FlowControl|DoOnce true
    (:Completed
      (Default|CloseDoor (Variables|Default|GetDoorRef))
      (Rendering|Material|SetScalarParameterValueonMaterials (Variables|Default|GetButton) "Emissive" 0.0)
      (Rendering|Material|SetScalarParameterValueonMaterials (Variables|Default|GetButtonBase) "Emissive" 0.0)
      (CallFunction|ResetOpen))))

(event Custom|ResetOpen
  (Utilities|FlowControl|DoOnce false) ; enters at Reset
)

(event Custom|ResetClose
  (Utilities|FlowControl|DoOnce true) ; enters at Reset
)

(event Custom|FoundDoor
  (Utilities|Array|ForEachLoopwithBreak (stale EventBeginPlay _outactors)) ; enters at Break
)

(event EventTick
  (params (DeltaSeconds :type Float%20%28single-precision%29))
  (Physics|SetPhysicsLinearVelocity (Variables|Default|GetButton) "0, 0,9.800000" true "None"))

(event EventBeginPlay
  (bind _outactors (Actor|GetAllActorsOfClass "/Game/Blueprint/Door.Door_C"))
  (bind _array_element (Utilities|Array|ForEachLoopwithBreak _outactors)
    (:LoopBody
      (if (== (Variables|/Game/Blueprint/Door.Door_C|GetDoorID _array_element) (Variables|Default|GetBottonID))
        (Variables|Default|SetDoorRef _array_element)
        (CallFunction|FoundDoor)))))

(fn ConstructionScript)
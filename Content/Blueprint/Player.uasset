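; First-person player character that moves, jumps, toggles crouch, fires low- or high-mass bullets and manipulates physics boxes.
; A per-tick camera trace highlights the targeted TheBox and marks it grabbable, using two cross-resetting DoOnce gates to act only on changes.
; A PhysicsHandle holds boxes under a mass limit ahead of the camera, then drops or throws them with mass-scaled force.
; KnockBack launches the character along a given impulse.
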(event Custom|DrobObject
  ;[1 1 1] Pick And Drop Object
  (Physics|Components|PhysicsHandle|ReleaseComponent (Variables|Default|GetPhysicsHandle))
  (Variables|Default|SetisHoldingObject false))

(event Custom|DeHighlight_Trigger
  ;[1 1 1] Highligth Box And Set Current Box
  (Utilities|FlowControl|DoOnce false) ; enters at Reset
)

(event Custom|PickUpObject
  (bind _currentbox (Variables|Default|GetCurrentBox))
  (bind _boxmesh (Variables|/Game/Blueprint/TheBox.TheBox_C|GetBoxMesh _currentbox))
  ;[1 1 1] Pick And Drop Object
  (Transformation|SetWorldRotation _boxmesh "0, 0, 0" false true)
  (Physics|Components|PhysicsHandle|GrabComponentatLocationwithRotation (Variables|Default|GetPhysicsHandle) _boxmesh "None" (Transformation|GetWorldLocation _boxmesh) "0, 0, 0")
  (Variables|Default|SetisHoldingObject true))

(event Custom|EveryTick_0
  (bind _returnvalue (Pawn|GetControlRotation :!class /Script/Engine.Pawn))
  (bind (_roll _pitch _yaw) (Math|Rotator|BreakRotator _returnvalue))
  (Class|PhysicsHandleComponent|SetTargetLocationandRotation (Variables|Default|GetPhysicsHandle) (+ (Transformation|GetWorldLocation (Variables|Default|GetCamera)) (* (Math|Vector|GetForwardVector _returnvalue) 2.2e+02)) (Math|Rotator|MakeRotator _roll 0.0 _yaw)))

(event Custom|EveryTick_1
  (bind _camera (Variables|Default|GetCamera))
  (bind _returnvalue (Transformation|GetWorldLocation _camera))
  ;[1 1 1] Highligth Box And Set Current Box
  (bind (_outhit _returnvalue_2) (Collision|LineTraceByChannel _returnvalue (+ _returnvalue (* (Math|Vector|GetForwardVector _camera) 3e+02)) "TraceTypeQuery1" false 0 "ForOneFrame" true "(R=1.000000,G=0.000000,B=0.000000,A=1.000000)" "(R=0.000000,G=1.000000,B=0.000000,A=1.000000)" 1e+01))
  (if _returnvalue_2
    (bind _asthe_box (Utilities|Casting|CastToTheBox (.HitActor (Collision|BreakHitResult _outhit)))
      (:then
        (Utilities|FlowControl|DoOnce false
          (:Completed
            (bind _output_get (Variables|Default|SetCurrentBox _asthe_box))
            (Default|Highlight _output_get)
            (Variables|Default|SetisCanGrab true)
            (CallFunction|DeHighlightTrigger))))
      (:CastFailed
        (Utilities|FlowControl|DoOnce false :!label _label
          (:Completed
            (if (!= (Variables|Default|GetCurrentBox) (Variables|Default|GetNullBox))
              (Default|DeHighlight (Variables|Default|GetCurrentBox))
              (Variables|Default|SetisCanGrab false)
              (CallFunction|HighlightTrigger))))))
    (else
      (goto _label))))

(event Custom|Highlight_Trigger
  ;[1 1 1] Highligth Box And Set Current Box
  (Utilities|FlowControl|DoOnce false) ; enters at Reset
)

(event EventBeginPlay)

(event Collision|EventActorBeginOverlap
  (params (OtherActor :type Actor%20Object%20Reference)))

(event EventTick
  (params (DeltaSeconds :type Float%20%28single-precision%29))
  (CallFunction|EveryTick0)
  (CallFunction|EveryTick1))

(event Input|ActionEvents|InputActionJump
  (params (Key :type Key%20Structure :default "AnyKey"))
  ;[1 1 1] Player Action Control
  (:Pressed
    (Character|Jump)))

(event Input|ActionEvents|InputActionCrouch
  (params (Key :type Key%20Structure :default "AnyKey"))
  ;[1 1 1] Player Action Control
  (:Pressed
    (if (Variables|Default|GetisCrouch)
      (Character|UnCrouch)
      (Variables|Default|SetisCrouch false)
      (else
        (Character|Crouch)
        (Variables|Default|SetisCrouch true)))))

(event Input|ActionEvents|InputActionPick_Drop_Object
  (params (Key :type Key%20Structure :default "AnyKey"))
  ;[1 1 1] Pick And Drop Object
  (:Pressed
    (if (Variables|Default|GetisHoldingObject)
      (CallFunction|DrobObject)
      (elif (Variables|Default|GetisCanGrab)
        (if (<= (Physics|GetMass (Variables|/Game/Blueprint/TheBox.TheBox_C|GetBoxMesh (Variables|Default|GetCurrentBox))) 1001.0)
          (CallFunction|PickUpObject))))))

(event Input|ActionEvents|InputActionThrow_Object
  (params (Key :type Key%20Structure :default "AnyKey"))
  ;[1 1 1] Throw Object
  (:Pressed
    (if (Variables|Default|GetisHoldingObject)
      (Physics|Components|PhysicsHandle|ReleaseComponent (Variables|Default|GetPhysicsHandle))
      (Default|ThrowObj (Variables|Default|GetCurrentBox) (* (Math|Vector|GetForwardVector (Variables|Default|GetCamera)) (/ (Variables|Default|GetForce) (Physics|GetMass (Variables|/Game/Blueprint/TheBox.TheBox_C|GetBoxMesh (Variables|Default|GetCurrentBox))))))
      (Variables|Default|SetisHoldingObject false))))

(event Input|AxisEvents|InputAxisMove_Forward_Backward
  (params (AxisValue :type Float%20%28single-precision%29))
  ;[1 1 1] Player Movement
  (Pawn|Input|AddMovementInput (Math|Vector|GetForwardVector (Math|Rotator|MakeRotator 0.0 0.0 (.Yaw (Math|Rotator|BreakRotator (Pawn|GetControlRotation :!class /Script/Engine.Pawn))))) AxisValue false))

(event Input|AxisEvents|InputAxisLook_Up_Down
  (params (AxisValue :type Float%20%28single-precision%29))
  ;[1 1 1] Player Look (Camera Control)
  (Pawn|Input|AddControllerPitchInput AxisValue))

(event Input|AxisEvents|InputAxisLook_Left_Right
  (params (AxisValue :type Float%20%28single-precision%29))
  ;[1 1 1] Player Look (Camera Control)
  (Pawn|Input|AddControllerYawInput AxisValue))

(event Input|AxisEvents|InputAxisMove_Left_Right
  (params (AxisValue :type Float%20%28single-precision%29))
  ;[1 1 1] Player Movement
  (Pawn|Input|AddMovementInput (Math|Vector|GetRightVector (Math|Rotator|MakeRotator 0.0 0.0 (.Yaw (Math|Rotator|BreakRotator (Pawn|GetControlRotation :!class /Script/Engine.Pawn))))) AxisValue false))

(event Input|MouseEvents|LeftMouseButton
  (params (Key :type Key%20Structure :default "AnyKey"))
  (bind _camera (Variables|Default|GetCamera))
  ;[1 1 1] Player Grove Action (Fire Bullet)
  (:Pressed
    (Game|SpawnActorfromClass "/Game/Blueprint/LowMassBullet.LowMassBullet_C" (Math|Transform|MakeTransform (Transformation|GetWorldLocation _camera) (Transformation|GetWorldRotation _camera)) "Undefined" 0 0)))

(event Input|MouseEvents|RightMouseButton
  (params (Key :type Key%20Structure :default "AnyKey"))
  (bind _camera (Variables|Default|GetCamera))
  ;[1 1 1] Player Grove Action (Fire Bullet)
  (:Pressed
    (Game|SpawnActorfromClass "/Game/Blueprint/HighMassBullet.HighMassBullet_C" (Math|Transform|MakeTransform (Transformation|GetWorldLocation _camera) (Transformation|GetWorldRotation _camera)) "Undefined" 0 0)))

(fn ConstructionScript)

(fn KnockBack
  (params (Normal%20Impulse :type Vector))
  (Character|LaunchCharacter (* Normal%20Impulse 5e+02) false false))
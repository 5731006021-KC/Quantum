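; Puzzle laser beam actor that activates switches and boxes it hits and knocks back players who touch it.
; Each tick it traces forward, ignoring its Box or BeamSource owner, and sets the beam endpoint at the hit.
; Macros track hit type to activate or deactivate targets, with box form also allowing destruction of wooden boxes.
; Two side collision components stretch to beam length and drive the knockback.
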(event OnComponentHit(LaserCollision_Right)
  (params (HitComponent :type Primitive%20Component%20Object%20Reference) (OtherActor :type Actor%20Object%20Reference) (OtherComp :type Primitive%20Component%20Object%20Reference) (NormalImpulse :type Vector) (Hit :type Hit%20Result%20Structure%20%28by%20ref%29))
  (bind _aspuzzle_player (Utilities|Casting|CastToPuzzlePlayer OtherActor))
  (Default|KnockBack _aspuzzle_player (Math|Vector|GetRightVector (Variables|Default|GetLaserCollision_Right))))

(event OnComponentHit(LaserCollision_Left)
  (params (HitComponent :type Primitive%20Component%20Object%20Reference) (OtherActor :type Actor%20Object%20Reference) (OtherComp :type Primitive%20Component%20Object%20Reference) (NormalImpulse :type Vector :default "0, 0, 0") (Hit :type Hit%20Result%20Structure%20%28by%20ref%29))
  (bind _aspuzzle_player (Utilities|Casting|CastToPuzzlePlayer OtherActor))
  (Default|KnockBack _aspuzzle_player (Math|Vector|GetRightVector (Variables|Default|GetLaserCollision_Left))))

(event Custom|Ignore%20Owner
  (bind _ownerobject (Variables|Default|GetOwnerObject))
  (bind _asbox (Utilities|Casting|CastToBox _ownerobject)
    (:CastFailed
      (bind _asbeam_source (Utilities|Casting|CastToBeamSource _ownerobject)))))

(event Collision|EventActorBeginOverlap
  (params (OtherActor :type Actor%20Object%20Reference)))

(event EventTick
  (params (DeltaSeconds :type Float%20%28single-precision%29))
  (bind _laserdirection (Variables|Default|GetLaserDirection))
  (bind _returnvalue (Transformation|GetWorldLocation _laserdirection))
  (bind _output_get (Variables|Default|SetEndPoint (+ _returnvalue (* (Math|Vector|GetForwardVector _laserdirection) 5e+03))))
  (bind (_outhit _returnvalue_2) (Collision|LineTraceByChannel _returnvalue _output_get "TraceTypeQuery1" false (Utilities|Array|MakeArray (stale Custom|Ignore%20Owner _asbeam_source) (stale Custom|Ignore%20Owner _asbox)) "ForOneFrame" true "(R=1.000000,G=0.000000,B=0.000000,A=1.000000)" "(R=0.133482,G=0.000000,B=1.000000,A=1.000000)"))
  (if _returnvalue_2
    (Variables|Default|SetEndPoint (.Location (Collision|BreakHitResult _outhit)))
    (bind (_boxactor _asswitch) (Utilities|HitObjectType (.HitActor (Collision|BreakHitResult _outhit)))
      (:HitBox
        (|HitBox _boxactor
          (:Out
            _)))
      (:HitSwitch
        (|HitSwitch _asswitch
          (:Out
            _)))
      (:HitOther
        (|HitOther :!label _label
          (:Out
            _))))
    (else
      (goto _label)))
  (Class|ParticleSystemComponent|SetBeamEndPoint (Variables|Default|GetLaserBeam) 0 (Variables|Default|GetEndPoint))
  (|ActivateCollision))

(fn ConstructionScript)
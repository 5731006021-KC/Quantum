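; Forcefield actor that pushes the player and TheBox objects upward while they are inside its overlap volume.
; Every Tick it polls overlapping actors, launching Player with a vertical velocity override and overwriting the box mesh's physics velocity.
; The construction script sets the volume's Z scale from ForceFieldHight.
; IncreasForce increments ForceLevel and multiplies the height by it, making the field taller without changing push strength.
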(event EventBeginPlay)

(event EventTick
  (params (DeltaSeconds :type Float%20%28single-precision%29))
  (for _array_element (Collision|GetOverlappingActors (Variables|Default|GetForceFieldOverlap) 0 :!class /Script/Engine.PrimitiveComponent)
    (bind _asplayer (Utilities|Casting|CastToPlayer _array_element)
      (:then
        (Character|LaunchCharacter _asplayer "0, 0,500.000000" false true))
      (:CastFailed
        (bind _asthe_box (Utilities|Casting|CastToTheBox _array_element))
        (Physics|SetPhysicsLinearVelocity (Variables|/Game/Blueprint/TheBox.TheBox_C|GetBoxMesh _asthe_box) "0, 0,980.000000" false "None")))))

(fn ConstructionScript
  (bind _forcefieldoverlap (Variables|Default|GetForceFieldOverlap))
  (bind _relativescale3d (Variables|/Script/Engine.SceneComponent|GetRelativeScale3D _forcefieldoverlap))
  (bind (_x _y) (Math|Vector|BreakVector _relativescale3d))
  (Transformation|SetRelativeScale3D _forcefieldoverlap (Math|Vector|MakeVector _x _y (Variables|Default|GetForceFieldHight))))

(fn IncreasForce
  (bind _forcefieldoverlap (Variables|Default|GetForceFieldOverlap))
  (bind _relativescale3d (Variables|/Script/Engine.SceneComponent|GetRelativeScale3D _forcefieldoverlap))
  (bind (_x _y) (Math|Vector|BreakVector _relativescale3d))
  (bind _result (Math|Float|IncrementFloat (Variables|Default|GetForceLevel))
    (:%20%20
      (Variables|Default|SetForceFieldHight (* _result (Variables|Default|GetForceFieldHight)))
      (Transformation|SetRelativeScale3D _forcefieldoverlap (Math|Vector|MakeVector _x _y (Variables|Default|GetForceFieldHight))))))
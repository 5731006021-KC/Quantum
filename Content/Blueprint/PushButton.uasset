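; Push button actor that triggers the BoxGenerator whose BoxGenID matches its PushBottonID, looked up at BeginPlay.
; A press plays an emissive timeline on the button and calls the generator's Process on the first update.
; Two DoOnce gates block repeat presses and repeat Process calls until the timeline finishes and resets them.
; Highlight and DeHighlight toggle render custom depth on the button.
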(event Custom|Event_Being_Press
  (Utilities|FlowControl|DoOnce false
    (:Completed
      (bind _emissive (Timeline|Emissive PlayFromStart)
        (:Update
          (Rendering|Material|SetScalarParameterValueonMaterials (Variables|Default|GetPushButton) "Emissive" (Math|Float|Lerp 0.0 1.0 _emissive))
          (Utilities|FlowControl|DoOnce false
            (:Completed
              (Default|Process (Variables|Default|GetBoxGenRef)))))
        (:Finished
          (Rendering|Material|SetScalarParameterValueonMaterials (Variables|Default|GetPushButton) "Emissive" 0.0)
          (CallFunction|ResetPush))))))

(event Custom|ResetPush
  (Utilities|FlowControl|Sequence
    (:then_0
      (Utilities|FlowControl|DoOnce false) ; enters at Reset
    )
    (:then_1
      (Utilities|FlowControl|DoOnce false) ; enters at Reset
    )))

(event Custom|FoundBoxGen
  (Utilities|Array|ForEachLoopwithBreak (stale EventBeginPlay _outactors)) ; enters at Break
)

(event EventBeginPlay
  (bind _outactors (Actor|GetAllActorsOfClass "/Game/Blueprint/BoxGenerator.BoxGenerator_C"))
  (bind _array_element (Utilities|Array|ForEachLoopwithBreak _outactors)
    (:LoopBody
      (if (== (Variables|/Game/Blueprint/BoxGenerator.BoxGenerator_C|GetBoxGenID _array_element) (Variables|Default|GetPushBottonID))
        (Variables|Default|SetBoxGenRef _array_element)
        (CallFunction|FoundBoxGen)))))

(event Collision|EventActorBeginOverlap
  (params (OtherActor :type Actor%20Object%20Reference)))

(event EventTick
  (params (DeltaSeconds :type Float%20%28single-precision%29)))

(event EventHighlight
  (if (not (Variables|Default|GetIsSetRenderDepth))
    (Rendering|SetRenderCustomDepth (Variables|Default|GetPushButton) true)
    (Variables|Default|SetIsSetRenderDepth true)))

(event EventDeHighlight
  (if (Variables|Default|GetIsSetRenderDepth)
    (Rendering|SetRenderCustomDepth (Variables|Default|GetPushButton) false)
    (Variables|Default|SetIsSetRenderDepth false)))

(fn ConstructionScript)
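; Platform actor that moves vertically when play begins, starting from its placed position.
; BeginPlay caches the component's world location and computes an end point offset by an EndZ height.
; An ActivatePlatform timeline then lerps the Platform component between the two points without sweep.
; Overlap, Tick and construction script are empty.
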(event EventBeginPlay
  (bind _platform (Variables|Default|GetPlatform))
  (bind _returnvalue (Transformation|GetWorldLocation _platform))
  (Variables|Default|SetEndLoc (+ (Math|Vector|MakeVector 0.0 0.0 (Variables|Default|GetEndZ)) _returnvalue))
  (Variables|Default|SetStartLoc _returnvalue)
  (bind _platformlerp (Timeline|ActivatePlatform Play)
    (:Update
      (Transformation|SetWorldLocation (Variables|Default|GetPlatform) (Math|Vector|Lerp(Vector) (Variables|Default|GetStartLoc) (Variables|Default|GetEndLoc) _platformlerp) false false))))

(event Collision|EventActorBeginOverlap
  (params (OtherActor :type Actor%20Object%20Reference)))

(event EventTick
  (params (DeltaSeconds :type Float%20%28single-precision%29)))

(fn ConstructionScript)
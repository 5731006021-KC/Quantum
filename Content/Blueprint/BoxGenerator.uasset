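; BoxGenerator is an actor that spawns TheBox actors and runs an animated BoxMechanism.
; On BeginPlay it attaches BoxCollision to the mechanism's Push socket, and Process unpauses the mechanism's animations.
; CreateBox destroys any existing box and spawns a half-scale replacement at the BoxGenerator component's location.
; CreateBoxCore toggles a skeletal mesh component, destroying a valid one or otherwise adding one.
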(event EventBeginPlay
  (Transformation|AttachComponentToComponent (Variables|Default|GetBoxCollision) (Variables|Default|GetBoxMechanism) "Push" "KeepWorld" "KeepWorld" "KeepWorld" false))

(event Collision|EventActorBeginOverlap
  (params (OtherActor :type Actor%20Object%20Reference)))

(event EventTick
  (params (DeltaSeconds :type Float%20%28single-precision%29)))

(fn ConstructionScript)

(fn Process
  (Variables|/Script/Engine.SkeletalMeshComponent|SetbPauseAnims (Variables|Default|GetBoxMechanism) false))

(fn CreateBox
  (Utilities|IsValid (Variables|Default|GetBoxRef)
    (:Is%20Valid
      (Default|DestroyBox (Variables|Default|GetBoxRef)))
    (:Is%20Not%20Valid
      _))
  (bind _returnvalue (Game|SpawnActorfromClass "/Game/Blueprint/TheBox.TheBox_C" (Math|Transform|MakeTransform (Transformation|GetWorldLocation (Variables|Default|GetBoxGenerator)) "0, 0, 0" "0.500000,0.500000,0.500000") "Undefined" 0 0))
  (Variables|Default|SetBoxRef _returnvalue))

(fn CreateBoxCore
  (Utilities|IsValid (Variables|Default|GetBoxCoreRef)
    (:Is%20Valid
      (Components|DestroyComponent (Variables|Default|GetBoxCoreRef)))
    (:Is%20Not%20Valid
      (bind _returnvalue (AddComponent|AddSkeletalMeshComponent false (Math|Transform|MakeTransform "0, 0, 0" "0, 0, 0" "1.000000,1.000000,1.000000")))
      (Variables|Default|SetBoxCoreRef _returnvalue))))
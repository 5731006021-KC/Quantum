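; Game mode for a puzzle game that handles player respawning and tracks play time in the game instance on Tick.
; BeginPlay and Respawn share setup that binds player destruction, adds a ShowTime widget, and loads TimePlay from the "Player" save or creates that save.
; On destruction, it briefly waits, spawns and possesses a new player at the game instance's SpawnTransform, then repeats the whole setup.
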(event Custom|Respawn
  (bind _aspuzzle_player (Utilities|Casting|CastToPuzzlePlayer (Game|GetPlayerCharacter 0)))
  (Game|BindEventtoOnDestroyed _aspuzzle_player (delegate Custom|OnDestroyed_Event))
  (bind _returnvalue (UserInterface|CreateWidget "/Game/Blueprint/Widget/ShowTime.ShowTime_C"))
  (UserInterface|Viewport|AddtoViewport _returnvalue 0)
  (bind _aspuzzle_game_instance (Utilities|Casting|CastToPuzzleGameInstance (Game|GetGameInstance)))
  (Variables|Default|SetGameInstance _aspuzzle_game_instance)
  (bind _returnvalue_2 (SaveGame|DoesSaveGameExist "Player"))
  (if _returnvalue_2
    (bind _returnvalue_3 (SaveGame|LoadGamefromSlot "Player"))
    (bind _asmy_save_game (Utilities|Casting|CastToMySaveGame _returnvalue_3))
    (Variables|/Game/Blueprint/PuzzleGameInstance.PuzzleGameInstance_C|SetTimePlay (Variables|Default|GetGameInstance) (Variables|/Game/Blueprint/MySaveGame.MySaveGame_C|GetTimePlay _asmy_save_game))
    (else
      (bind _returnvalue_4 (SaveGame|CreateSaveGameObject "/Game/Blueprint/MySaveGame.MySaveGame_C"))
      (bind _output_get (Variables|Default|SetSaveGameInstance _returnvalue_4))
      (bind _asmy_save_game_2 (Utilities|Casting|CastToMySaveGame _output_get))
      (SaveGame|SaveGametoSlot _asmy_save_game_2 "Player"))))

(event Custom|OnDestroyed_Event
  (params (DestroyedActor :type Actor%20Object%20Reference))
  (bind _aspuzzle_game_instance (Utilities|Casting|CastToPuzzleGameInstance (Game|GetGameInstance)))
  (Utilities|FlowControl|Delay 0.2)
  (bind _returnvalue (Game|SpawnActorfromClass "/Game/Blueprint/PuzzlePlayer.PuzzlePlayer_C" (Variables|/Game/Blueprint/PuzzleGameInstance.PuzzleGameInstance_C|GetSpawnTransform _aspuzzle_game_instance) "Undefined" 0 0))
  (Pawn|Possess (Game|GetPlayerController 0) _returnvalue)
  (CallFunction|Respawn))

(event EventBeginPlay
  (bind _aspuzzle_player (Utilities|Casting|CastToPuzzlePlayer (Game|GetPlayerCharacter 0)))
  (Game|BindEventtoOnDestroyed _aspuzzle_player (delegate Custom|OnDestroyed_Event))
  (bind _returnvalue (UserInterface|CreateWidget "/Game/Blueprint/Widget/ShowTime.ShowTime_C"))
  (UserInterface|Viewport|AddtoViewport _returnvalue 0)
  (bind _aspuzzle_game_instance (Utilities|Casting|CastToPuzzleGameInstance (Game|GetGameInstance)))
  (Variables|Default|SetGameInstance _aspuzzle_game_instance)
  (bind _returnvalue_2 (SaveGame|DoesSaveGameExist "Player"))
  (if _returnvalue_2
    (bind _returnvalue_3 (SaveGame|LoadGamefromSlot "Player"))
    (bind _asmy_save_game (Utilities|Casting|CastToMySaveGame _returnvalue_3))
    (Variables|/Game/Blueprint/PuzzleGameInstance.PuzzleGameInstance_C|SetTimePlay (Variables|Default|GetGameInstance) (Variables|/Game/Blueprint/MySaveGame.MySaveGame_C|GetTimePlay _asmy_save_game))
    (else
      (bind _returnvalue_4 (SaveGame|CreateSaveGameObject "/Game/Blueprint/MySaveGame.MySaveGame_C"))
      (bind _output_get (Variables|Default|SetSaveGameInstance _returnvalue_4))
      (bind _asmy_save_game_2 (Utilities|Casting|CastToMySaveGame _output_get))
      (SaveGame|SaveGametoSlot _asmy_save_game_2 "Player"))))

(event EventTick
  (params (DeltaSeconds :type Float%20%28single-precision%29))
  (Variables|/Game/Blueprint/PuzzleGameInstance.PuzzleGameInstance_C|SetTimePlay (Variables|Default|GetGameInstance) (+ DeltaSeconds (Variables|/Game/Blueprint/PuzzleGameInstance.PuzzleGameInstance_C|GetTimePlay (Variables|Default|GetGameInstance)))))

(fn ConstructionScript)
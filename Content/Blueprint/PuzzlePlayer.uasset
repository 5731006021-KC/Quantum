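; First-person puzzle player character that moves, fires low and high mass bullets, and picks up, drops or throws boxes.
; A per-tick camera trace highlights interactables and sets the current box or button.
; Held boxes follow a PhysicsHandle through timer-driven lerp-in and hold states, auto-dropping when blocked or out of range too long.
; Escape saves play time and quits, while standing still for five seconds deletes the save and quits.
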(event Custom|DropObject
  (bind _liftingbox (Variables|Actor|GetLiftingBox))
  (bind _boxmesh (Variables|/Game/Blueprint/TheBox.TheBox_C|GetBoxMesh _liftingbox))
  ;[1 1 1] Pick And Drop Object
  (Physics|Components|PhysicsHandle|ReleaseComponent (Variables|Default|GetPhysicsHandle))
  (Variables|Default|SetisHoldingObject false)
  (Default|SetBackMass _liftingbox)
  (Class|PrimitiveComponent|SetAllPhysicsLinearVelocity _boxmesh "0, 0, 0" false)
  (Class|PrimitiveComponent|SetPhysicsAngularVelocity _boxmesh "0, 0, 0" false "None")
  (Collision|SetCollisionResponsetoChannel _boxmesh "ECC_GameTraceChannel1" "ECR_Ignore")
  (Collision|SetCollisionResponsetoChannel _boxmesh "ECC_GameTraceChannel2" "ECR_Ignore")
  (|IsObjectOutOfRange) ; enters at Release
)

(event Custom|PickUpObject
  ;[1 1 1] Pick And Drop Object
  (Variables|Actor|SetLiftingBox (Variables|Actor|GetCurrentBox))
  (Physics|Components|PhysicsHandle|GrabComponentatLocationwithRotation (Variables|Default|GetPhysicsHandle) (Variables|/Game/Blueprint/TheBox.TheBox_C|GetBoxMesh (Variables|Actor|GetLiftingBox)) "None" (Transformation|GetActorLocation (Variables|Actor|GetLiftingBox)) (Transformation|GetActorRotation (Variables|Actor|GetLiftingBox)))
  (Variables|Default|SetisHoldingObject true)
  (Class|PrimitiveComponent|SetMassOverrideinKg (Variables|/Game/Blueprint/TheBox.TheBox_C|GetBoxMesh (Variables|Actor|GetLiftingBox)) "None" 1.0 true)
  (Collision|SetCollisionResponsetoChannel (Variables|/Game/Blueprint/TheBox.TheBox_C|GetBoxMesh (Variables|Actor|GetLiftingBox)) "ECC_GameTraceChannel1" "ECR_Block")
  (Collision|SetCollisionResponsetoChannel (Variables|/Game/Blueprint/TheBox.TheBox_C|GetBoxMesh (Variables|Actor|GetLiftingBox)) "ECC_GameTraceChannel2" "ECR_Block")
  (|IsObjectOutOfRange))

(event Custom|EveryTick_0
  (bind _camera (Variables|Default|GetCamera))
  (bind _returnvalue (Transformation|GetWorldLocation _camera))
  ;[1 1 1] Highligth Box And Set Current Box
  (bind (_outhit _returnvalue_2) (Collision|LineTraceByChannel _returnvalue (+ _returnvalue (* (Math|Vector|GetForwardVector _camera) 2.5e+02)) "TraceTypeQuery1" false 0 "ForOneFrame" false "(R=1.000000,G=0.000000,B=0.000000,A=1.000000)" "(R=0.000000,G=1.000000,B=0.000000,A=1.000000)" 1e+01))
  (if _returnvalue_2
    (bind _asinteract_able (Utilities|Casting|CastToInteractAble (.HitActor (Collision|BreakHitResult _outhit)))
      (:then
        (if (!= (Utilities|ToObject(Interface) (Variables|Default|GetCurrentObj)) (Utilities|ToObject(Interface) _asinteract_able))
          (if (Variables|Default|GetIsCurrentObjAvailable)
            (Default|DeHighlight (Variables|Default|GetCurrentObj)))
          (bind _output_get (Variables|Default|SetCurrentObj _asinteract_able))
          (Default|Highlight _output_get)
          (Variables|Default|SetIsCurrentObjAvailable true)
          ;[1 1 1] Cast Parent To Child
          (bind _asthe_box (Utilities|Casting|CastToTheBox (Variables|Default|GetCurrentObj))
            (:then
              (Variables|Actor|SetCurrentBox _asthe_box)
              (Variables|Actor|SetCurrentPushButton 0))
            (:CastFailed
              (bind _aspush_button (Utilities|Casting|CastToPushButton (Variables|Default|GetCurrentObj))
                (:then
                  (Variables|Actor|SetCurrentPushButton _aspush_button)
                  (Variables|Actor|SetCurrentBox 0))
                (:CastFailed
                  (Variables|Actor|SetCurrentBox 0 :!label _label)
                  (Variables|Actor|SetCurrentPushButton 0)))))))
      (:CastFailed
        (if (Variables|Default|GetIsCurrentObjAvailable) :!label _label_2
          (Default|DeHighlight (Variables|Default|GetCurrentObj))
          (Variables|Default|SetCurrentObj 0)
          (Variables|Default|SetIsCurrentObjAvailable false)
          (goto _label))))
    (else
      (goto _label_2))))

(event EventTick
  (params (DeltaSeconds :type Float%20%28single-precision%29))
  (CallFunction|EveryTick0)
  (|SaveGame))

(event EventBeginPlay
  (bind _returnvalue (UserInterface|CreateWidget "/Game/Blueprint/Widget/Tutorial.Tutorial_C" (Game|GetPlayerController 0)))
  (bind _output_get (Variables|Default|SetWidget _returnvalue))
  (UserInterface|Viewport|AddtoViewport _output_get 0)
  (bind _aspuzzle_game_instance (Utilities|Casting|CastToPuzzleGameInstance (Game|GetGameInstance)))
  (Variables|Default|SetGameInstance _aspuzzle_game_instance))

(event Input|ActionEvents|InputActionJump
  (params (Key :type Key%20Structure :default "AnyKey"))
  ;[1 1 1] Player Action Control
  (:Pressed
    (Character|Jump)))

(event Input|ActionEvents|InputActionFire_LowMass
  (params (Key :type Key%20Structure :default "AnyKey"))
  (bind _camera (Variables|Default|GetCamera))
  (bind _returnvalue (Transformation|GetWorldLocation _camera))
  ;[1 1 1] Player Grove Action (Fire Bullet)
  (:Pressed
    (if (not (Variables|Default|GetisHoldingObject))
      (Audio|PlaySoundatLocation "/Game/SoundVFX/GunFire02.GunFire02" _returnvalue)
      (Game|SpawnActorfromClass "/Game/Blueprint/LowMassBullet.LowMassBullet_C" (Math|Transform|MakeTransform _returnvalue (Transformation|GetWorldRotation _camera) "1.000000,1,1") "Undefined" 0 0))))

(event Input|ActionEvents|InputActionFire_HighMass
  (params (Key :type Key%20Structure :default "AnyKey"))
  (bind _camera (Variables|Default|GetCamera))
  ;[1 1 1] Player Grove Action (Fire Bullet)
  (:Pressed
    (if (not (Variables|Default|GetisHoldingObject))
      (Game|SpawnActorfromClass "/Game/Blueprint/HighMassBullet.HighMassBullet_C" (Math|Transform|MakeTransform (Transformation|GetWorldLocation _camera) (Transformation|GetWorldRotation _camera)) "Undefined" 0 0))))

(event Input|ActionEvents|InputActionCrouch
  (params (Key :type Key%20Structure :default "AnyKey"))
  ;[1 1 1] Player Action Control
  (:Pressed
    (if (Variables|Default|GetisCrouch)
      (Character|UnCrouch)
      (Variables|Default|SetisCrouch false)
      (else
        (Character|Crouch)
        (Variables|Default|SetisCrouch true)))))

(event Input|ActionEvents|InputActionThrow_Object
  (params (Key :type Key%20Structure :default "AnyKey"))
  ;[1 1 1] Throw Object
  (:Pressed
    (if (Variables|Default|GetisHoldingObject)
      (CallFunction|DropObject)
      (if (Utilities|Enum|Equal(Enum) "NewEnumerator2" (Variables|/Game/Blueprint/TheBox.TheBox_C|GetTheBoxStatus (Variables|Actor|GetLiftingBox)))
        (Variables|Default|SetForce 1.5e+03)
        (else
          (Variables|Default|SetForce 2.5e+02)))
      (Default|ThrowObj (Variables|Actor|GetLiftingBox) (* (Math|Vector|GetForwardVector (Variables|Default|GetCamera)) (Variables|Default|GetForce)))
      (Variables|Actor|SetLiftingBox 0))))

(event Input|ActionEvents|InputActionInteract
  (params (Key :type Key%20Structure :default "AnyKey"))
  ;[1 1 1] Pick And Drop Object
  (:Pressed
    (if (not (Variables|Default|GetisHoldingObject))
      (Utilities|Casting|CastToTheBox (Variables|Default|GetCurrentObj)
        (:then
          (if (Utilities|Enum|NotEqual(Enum) "NewEnumerator0" (Variables|/Game/Blueprint/TheBox.TheBox_C|GetTheBoxStatus (Variables|Actor|GetCurrentBox)))
            (CallFunction|PickUpObject)))
        (:CastFailed
          (Utilities|Casting|CastToPushButton (Variables|Default|GetCurrentObj))
          (Default|EventBeingPress (Variables|Actor|GetCurrentPushButton))))
      (else
        (CallFunction|DropObject)
        (Variables|Actor|SetLiftingBox 0)))))

(event Input|AxisEvents|InputAxisMove_Forward_Backward
  (params (AxisValue :type Float%20%28single-precision%29))
  ;[1 1 1] Player Movement
  (Pawn|Input|AddMovementInput (Math|Vector|GetForwardVector (Math|Rotator|MakeRotator 0.0 0.0 (.Yaw (Math|Rotator|BreakRotator (Pawn|GetControlRotation :!class /Script/Engine.Pawn))))) AxisValue false))

(event Input|AxisEvents|InputAxisLook_Up_Down
  (params (AxisValue :type Float%20%28single-precision%29))
  ;[1 1 1] Player Look (Camera Control)
  (Pawn|Input|AddControllerPitchInput AxisValue))

(event Input|AxisEvents|InputAxisLook_Left_Right
  (params (AxisValue :type Float%20%28single-precision%29))
  ;[1 1 1] Player Look (Camera Control)
  (Pawn|Input|AddControllerYawInput AxisValue))

(event Input|AxisEvents|InputAxisMove_Left_Right
  (params (AxisValue :type Float%20%28single-precision%29))
  ;[1 1 1] Player Movement
  (Pawn|Input|AddMovementInput (Math|Vector|GetRightVector (Math|Rotator|MakeRotator 0.0 0.0 (.Yaw (Math|Rotator|BreakRotator (Pawn|GetControlRotation :!class /Script/Engine.Pawn))))) AxisValue false))

(event Input|MouseEvents|MiddleMouseButton
  (params (Key :type Key%20Structure :default "AnyKey"))
  ;[1 1 1] Player Grove Action (Fire Bullet)
  (:Pressed
    (if (not (Variables|Default|GetisHoldingObject))
      (Default|MediumMass (Variables|Actor|GetCurrentBox)))))

(event Input|KeyboardEvents|Q
  (params (Key :type Key%20Structure :default "AnyKey"))
  (:Pressed
    (Variables|/Game/Blueprint/PuzzleGameInstance.PuzzleGameInstance_C|SetSpawnTransform (Variables|Default|GetGameInstance) (Transformation|GetActorTransform))))

(event Input|KeyboardEvents|R
  (params (Key :type Key%20Structure :default "AnyKey"))
  (bind _widget (Variables|Default|GetWidget))
  (:Pressed
    (Utilities|FlowControl|FlipFlop
      (:A
        (Widget|SetVisibility _widget "Hidden"))
      (:B
        (Widget|SetVisibility _widget "Visible")))))

(fn ConstructionScript)

(fn KnockBack
  (params (Normal%20Impulse :type Vector))
  (Character|LaunchCharacter (* Normal%20Impulse 7e+02) true true))

(event Custom|IsObjBlock
  (Variables|IsObjectOutOfRange|SetTimerBlock (+ (Variables|IsObjectOutOfRange|GetTimerBlock) (Utilities|Time|GetWorldDeltaSeconds)))
  (if (>= (Variables|IsObjectOutOfRange|GetTimerBlock) (Variables|IsObjectOutOfRange|GetTimerBlockThreshold))
    (CallFunction|DropObject)
    (Variables|Actor|SetLiftingBox 0)))

(event Custom|StartState
  (if (< (Variables|IsObjectOutOfRange|GetTransformLerp) 1.0)
    (Variables|IsObjectOutOfRange|SetTransformLerp (Math|Float|Clamp(Float) (+ (Variables|IsObjectOutOfRange|GetTransformLerp) (Variables|IsObjectOutOfRange|GetTransformRate))))
    (Utilities|StartStatePhysicsHandleTransform)
    (else
      (Utilities|Time|PauseTimerbyHandle (Variables|IsObjectOutOfRange|GetCurrentStateHandle))
      (bind _returnvalue (Utilities|Time|SetTimerbyEvent (delegate Custom|NormalState) (Utilities|Time|GetWorldDeltaSeconds) true))
      (Variables|IsObjectOutOfRange|SetCurrentStateHandle _returnvalue)
      (CallFunction|AutoDropObj))))

(event Custom|IsObjOOR
  (Variables|IsObjectOutOfRange|SetTimerOOR (+ (Variables|IsObjectOutOfRange|GetTimerOOR) (Utilities|Time|GetWorldDeltaSeconds)))
  (if (>= (Variables|IsObjectOutOfRange|GetTimerOOR) (Variables|IsObjectOutOfRange|GetTimerOORThreshold))
    (CallFunction|DropObject)
    (Variables|Actor|SetLiftingBox 0)))

(event Custom|NormalState
  (Utilities|NormalStatePhysicsHandleTransform
    (:Out
      (CallFunction|AutoDropObj))))

(event Custom|AutoDropObj
  (bind _ishit (Utilities|LineTraceChannel (Variables|Default|GetCamera) (Variables|IsObjectOutOfRange|GetDropObjRange) "TraceTypeQuery4")
    (:Out
      (if _ishit
        (bind _hitresult (Utilities|LineTraceObject (Variables|Default|GetCamera) (Variables|/Game/Blueprint/TheBox.TheBox_C|GetBoxMesh (Variables|Actor|GetLiftingBox)) "TraceTypeQuery3")
          (:Out
            (if (!= (Variables|Actor|GetLiftingBox) (.HitActor (Collision|BreakHitResult _hitresult)))
              (CallFunction|IsObjBlock)
              (else
                (Variables|IsObjectOutOfRange|SetTimerBlock 0.0)))))
        (elif (and (Utilities|IsonViewport) (Utilities|IsOutOfRange))
          (Variables|IsObjectOutOfRange|SetTimerOOR 0.0)
          (else
            (CallFunction|IsObjOOR)))))))

(event Input|KeyboardEvents|Escape
  (params (Key :type Key%20Structure :default "AnyKey"))
  (:Pressed
    (bind _returnvalue (SaveGame|LoadGamefromSlot "Player"))
    (bind _output_get (Variables|SaveGame|SetSaveGameInstance _returnvalue))
    (bind _asmy_save_game (Utilities|Casting|CastToMySaveGame _output_get))
    (Variables|/Game/Blueprint/MySaveGame.MySaveGame_C|SetTimePlay _asmy_save_game (Variables|/Game/Blueprint/PuzzleGameInstance.PuzzleGameInstance_C|GetTimePlay (Variables|Default|GetGameInstance)))
    (SaveGame|SaveGametoSlot (Variables|SaveGame|GetSaveGameInstance) "Player")
    (Game|QuitGame 0 "Quit")))
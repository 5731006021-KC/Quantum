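; Laser actor that draws a particle beam between two points, with collision components fitted along it.
; Functions set the beam's start and end, and construction zeroes the end point; the event graph has no active logic.
; Two ScaleTriggerBox variants stretch LaserCollision from the beam's midpoint and put a small LaserCollisionExtend at the end.
; The LaserSource variant positions them with axis-swapped relative offsets, the TheBox variant in world space.
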(event EventBeginPlay)

(event EventTick
  (params (DeltaSeconds :type Float%20%28single-precision%29)))

(fn ConstructionScript
  (Class|ParticleSystemComponent|SetBeamEndPoint (Variables|Default|GetLaser) 0 "0.000000, 0, 0"))

(fn SetLaserEndPoint
  (params (EndPoint :type Vector))
  (Class|ParticleSystemComponent|SetBeamEndPoint (Variables|Default|GetLaser) 0 EndPoint))

(fn ScaleTriggerBox(LaserSource)
  (params (EndPoint :type Vector) (StartPoint :type Vector) (Rot :type Rotator))
  (bind _returnvalue (- EndPoint StartPoint))
  (bind (_roll _pitch _yaw) (Math|Rotator|BreakRotator Rot))
  (bind (_x _y _z) (Math|Vector|BreakVector _returnvalue))
  (bind _returnvalue_2 (- _yaw 2.7e+02))
  (bind _returnvalue_3 (/ _returnvalue 2.0))
  (bind (_x_2 _y_2 _z_2) (Math|Vector|BreakVector _returnvalue_3))
  (bind _returnvalue_4 (Math|Rotator|MakeRotator _roll _pitch _returnvalue_2))
  (Transformation|SetRelativeTransform (Variables|Default|GetLaserCollision) (Math|Transform|MakeTransform (Math|Vector|MakeVector (* _y_2 -1.0) _x_2 _z_2) _returnvalue_4 (Math|Vector|MakeVector 0.1 0.1 (/ (Math|Vector|VectorLength _returnvalue_3) 44.0))) false false)
  (Transformation|SetRelativeTransform (Variables|Default|GetLaserCollisionExtend) (Math|Transform|MakeTransform (Math|Vector|MakeVector (* _y -1.0) _x _z) _returnvalue_4 (Math|Vector|MakeVector 0.1 0.1 1.0)) false false))

(fn SetLaserStartPoint
  (params (StartPoint :type Vector))
  (Class|ParticleSystemComponent|SetBeamSourcePoint (Variables|Default|GetLaser) 0 StartPoint))

(fn ScaleTriggerBox(TheBox)
  (params (EndPoint :type Vector) (StartPoint :type Vector) (Rot :type Rotator))
  (bind _returnvalue (- EndPoint StartPoint))
  (bind (_roll _pitch _yaw) (Math|Rotator|BreakRotator Rot))
  (bind _returnvalue_2 (- _roll 9e+01))
  (bind _returnvalue_3 (/ _returnvalue 2.0))
  (bind _returnvalue_4 (Math|Rotator|MakeRotator _yaw _returnvalue_2 _pitch))
  (Transformation|SetRelativeRotation (Variables|Default|GetLaserCollision) _returnvalue_4 false false)
  (Transformation|SetRelativeRotation (Variables|Default|GetLaserCollisionExtend) _returnvalue_4 false false)
  (Transformation|SetRelativeScale3D (Variables|Default|GetLaserCollision) (Math|Vector|MakeVector 0.1 0.1 (/ (Math|Vector|VectorLength _returnvalue_3) 44.0)))
  (Transformation|SetRelativeScale3D (Variables|Default|GetLaserCollisionExtend) "0.100000,0.100000,1.000000")
  (Transformation|SetWorldLocation (Variables|Default|GetLaserCollision) (+ StartPoint _returnvalue_3) false false)
  (Transformation|SetWorldLocation (Variables|Default|GetLaserCollisionExtend) EndPoint false false))